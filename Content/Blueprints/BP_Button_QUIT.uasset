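; BP_Button_QUIT is a clickable in-world quit button built from two static mesh components that act as one control.
; Clicking either mesh calls QuitGame to exit the game.
; Cursor-over events on either mesh switch both to a brown material, and cursor-exit events switch both to gray for hover feedback.
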(event OnClicked(StaticMesh)
  (params (TouchedComponent :type Primitive%20Component%20Object%20Reference) (ButtonPressed :type Key%20Structure))
  (Game|QuitGame 0 "Quit" false))

(event OnClicked(StaticMesh1)
  (params (TouchedComponent :type Primitive%20Component%20Object%20Reference) (ButtonPressed :type Key%20Structure))
  (Game|QuitGame 0 "Quit" false))

(event OnBeginCursorOver(StaticMesh)
  (params (TouchedComponent :type Primitive%20Component%20Object%20Reference))
  (Rendering|Material|SetMaterial (Variables|Default|GetStaticMesh) 0 "/Game/Meshes/Brown_10.Brown_10")
  (Rendering|Material|SetMaterial (Variables|Default|GetStaticMesh1) 0 "/Game/Meshes/Brown_10.Brown_10"))

(event OnBeginCursorOver(StaticMesh1)
  (params (TouchedComponent :type Primitive%20Component%20Object%20Reference))
  (Rendering|Material|SetMaterial (Variables|Default|GetStaticMesh) 0 "/Game/Meshes/Brown_10.Brown_10")
  (Rendering|Material|SetMaterial (Variables|Default|GetStaticMesh1) 0 "/Game/Meshes/Brown_10.Brown_10"))

(event OnEndCursorOver(StaticMesh)
  (params (TouchedComponent :type Primitive%20Component%20Object%20Reference))
  (Rendering|Material|SetMaterial (Variables|Default|GetStaticMesh) 0 "/Game/Meshes/Gray_2.Gray_2")
  (Rendering|Material|SetMaterial (Variables|Default|GetStaticMesh1) 0 "/Game/Meshes/Gray_2.Gray_2"))

(event OnEndCursorOver(StaticMesh1)
  (params (TouchedComponent :type Primitive%20Component%20Object%20Reference))
  (Rendering|Material|SetMaterial (Variables|Default|GetStaticMesh) 0 "/Game/Meshes/Gray_2.Gray_2")
  (Rendering|Material|SetMaterial (Variables|Default|GetStaticMesh1) 0 "/Game/Meshes/Gray_2.Gray_2"))

(fn ConstructionScript
  (|CallParentFunction))