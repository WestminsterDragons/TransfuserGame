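; ShowEndL is an actor that displays end-of-level results on a set of 3D text render components.
; On BeginPlay it has the first-person player character calculate the score.
; It then writes timer, death, platform and total score figures from the Global game instance and the character's Score array into the text fields as integers.
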(event EventBeginPlay
  (bind _asfirst_person_character_ray_cast_prohress_bar (Utilities|Casting|CastToFirstPersonCharacterRayCast_ProhressBar (Game|GetPlayerCharacter 0)))
  (bind _asglobal (Utilities|Casting|CastToGlobal (Game|GetGameInstance)))
  (Default|CalculateScore _asfirst_person_character_ray_cast_prohress_bar)
  (Utilities|FlowControl|Sequence
    (:then_0
      (Rendering|Components|TextRender|SetText (Variables|/Script/Engine.TextRenderActor|GetTextRender (Variables|Default|GetText)) (Utilities|Text|ToText(Integer) (Variables|/Game/Blueprints/Global.Global_C|GetTimer _asglobal))))
    (:then_1
      (Rendering|Components|TextRender|SetText (Variables|/Script/Engine.TextRenderActor|GetTextRender (Variables|Default|GetText_0)) (Utilities|Text|ToText(Integer) (Variables|/Game/Blueprints/Global.Global_C|GetTimerValue _asglobal))))
    (:then_2
      (Rendering|Components|TextRender|SetText (Variables|/Script/Engine.TextRenderActor|GetTextRender (Variables|Default|GetText_1)) (Utilities|Text|ToText(Integer) (Utilities|Array|Get(acopy) (Variables|/Game/Blueprints/FirstPersonCharacterRayCast_ProhressBar.FirstPersonCharacterRayCast_ProhressBar_C|GetScore _asfirst_person_character_ray_cast_prohress_bar) 1))))
    (:then_3
      (Rendering|Components|TextRender|SetText (Variables|/Script/Engine.TextRenderActor|GetTextRender (Variables|Default|GetText_2)) (Utilities|Text|ToText(Integer) (Variables|/Game/Blueprints/Global.Global_C|GetDeath _asglobal))))
    (:then_4
      (Rendering|Components|TextRender|SetText (Variables|/Script/Engine.TextRenderActor|GetTextRender (Variables|Default|GetText_3)) (Utilities|Text|ToText(Integer) (Utilities|Array|Get(acopy) (Variables|/Game/Blueprints/FirstPersonCharacterRayCast_ProhressBar.FirstPersonCharacterRayCast_ProhressBar_C|GetScore _asfirst_person_character_ray_cast_prohress_bar)))))
    (:then_5
      (Rendering|Components|TextRender|SetText (Variables|/Script/Engine.TextRenderActor|GetTextRender (Variables|Default|GetText_4)) (Utilities|Text|ToText(Integer) (Variables|/Game/Blueprints/Global.Global_C|GetPlatform _asglobal))))
    (:then_6
      (Rendering|Components|TextRender|SetText (Variables|/Script/Engine.TextRenderActor|GetTextRender (Variables|Default|GetText_5)) (Utilities|Text|ToText(Integer) (Variables|/Game/Blueprints/FirstPersonCharacterRayCast_ProhressBar.FirstPersonCharacterRayCast_ProhressBar_C|GetPlattformValue _asfirst_person_character_ray_cast_prohress_bar))))
    (:then_7
      (Rendering|Components|TextRender|SetText (Variables|/Script/Engine.TextRenderActor|GetTextRender (Variables|Default|GetText_6)) (Utilities|Text|ToText(Integer) (Utilities|Array|Get(acopy) (Variables|/Game/Blueprints/FirstPersonCharacterRayCast_ProhressBar.FirstPersonCharacterRayCast_ProhressBar_C|GetScore _asfirst_person_character_ray_cast_prohress_bar) 2))))
    (:then_8
      (Rendering|Components|TextRender|SetText (Variables|/Script/Engine.TextRenderActor|GetTextRender (Variables|Default|GetText_7)) (Utilities|Text|ToText(Integer) (Variables|/Game/Blueprints/Global.Global_C|GetScore _asglobal))))))

(fn ConstructionScript)