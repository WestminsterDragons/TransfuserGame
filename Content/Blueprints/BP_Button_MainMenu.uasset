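; Clickable in-world main menu button built from four static meshes that act as one control.
; Clicking any of the meshes opens the MainMenu level by name.
; Cursor hover on any mesh swaps all four to a brown highlight material, and leaving restores gray, with every mesh's events routed into shared handlers.
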(event OnClicked(StaticMesh)
  (params (TouchedComponent :type Primitive%20Component%20Object%20Reference) (ButtonPressed :type Key%20Structure))
  (Game|OpenLevel(byName) "MainMenu"))

(event OnClicked(StaticMesh1)
  (params (TouchedComponent :type Primitive%20Component%20Object%20Reference) (ButtonPressed :type Key%20Structure))
  (Game|OpenLevel(byName) "MainMenu"))

(event OnEndCursorOver(StaticMesh2)
  (params (TouchedComponent :type Primitive%20Component%20Object%20Reference))
  (Rendering|Material|SetMaterial (Variables|Default|GetStaticMesh) 0 "/Game/Materials/Gray_2.Gray_2")
  (Rendering|Material|SetMaterial (Variables|Default|GetStaticMesh1) 0 "/Game/Materials/Gray_2.Gray_2")
  (Rendering|Material|SetMaterial (Variables|Default|GetStaticMesh2) 0 "/Game/Materials/Gray_2.Gray_2")
  (Rendering|Material|SetMaterial (Variables|Default|GetStaticMesh3) 0 "/Game/Materials/Gray_2.Gray_2"))

(event OnEndCursorOver(StaticMesh3)
  (params (TouchedComponent :type Primitive%20Component%20Object%20Reference))
  (Rendering|Material|SetMaterial (Variables|Default|GetStaticMesh) 0 "/Game/Materials/Gray_2.Gray_2")
  (Rendering|Material|SetMaterial (Variables|Default|GetStaticMesh1) 0 "/Game/Materials/Gray_2.Gray_2")
  (Rendering|Material|SetMaterial (Variables|Default|GetStaticMesh2) 0 "/Game/Materials/Gray_2.Gray_2")
  (Rendering|Material|SetMaterial (Variables|Default|GetStaticMesh3) 0 "/Game/Materials/Gray_2.Gray_2"))

(event OnBeginCursorOver(StaticMesh)
  (params (TouchedComponent :type Primitive%20Component%20Object%20Reference))
  (Rendering|Material|SetMaterial (Variables|Default|GetStaticMesh) 0 "/Game/Materials/Brown_10.Brown_10")
  (Rendering|Material|SetMaterial (Variables|Default|GetStaticMesh1) 0 "/Game/Materials/Brown_10.Brown_10")
  (Rendering|Material|SetMaterial (Variables|Default|GetStaticMesh2) 0 "/Game/Materials/Brown_10.Brown_10")
  (Rendering|Material|SetMaterial (Variables|Default|GetStaticMesh3) 0 "/Game/Materials/Brown_10.Brown_10"))

(event OnBeginCursorOver(StaticMesh1)
  (params (TouchedComponent :type Primitive%20Component%20Object%20Reference))
  (Rendering|Material|SetMaterial (Variables|Default|GetStaticMesh) 0 "/Game/Materials/Brown_10.Brown_10")
  (Rendering|Material|SetMaterial (Variables|Default|GetStaticMesh1) 0 "/Game/Materials/Brown_10.Brown_10")
  (Rendering|Material|SetMaterial (Variables|Default|GetStaticMesh2) 0 "/Game/Materials/Brown_10.Brown_10")
  (Rendering|Material|SetMaterial (Variables|Default|GetStaticMesh3) 0 "/Game/Materials/Brown_10.Brown_10"))

(event OnEndCursorOver(StaticMesh)
  (params (TouchedComponent :type Primitive%20Component%20Object%20Reference))
  (Rendering|Material|SetMaterial (Variables|Default|GetStaticMesh) 0 "/Game/Materials/Gray_2.Gray_2")
  (Rendering|Material|SetMaterial (Variables|Default|GetStaticMesh1) 0 "/Game/Materials/Gray_2.Gray_2")
  (Rendering|Material|SetMaterial (Variables|Default|GetStaticMesh2) 0 "/Game/Materials/Gray_2.Gray_2")
  (Rendering|Material|SetMaterial (Variables|Default|GetStaticMesh3) 0 "/Game/Materials/Gray_2.Gray_2"))

(event OnEndCursorOver(StaticMesh1)
  (params (TouchedComponent :type Primitive%20Component%20Object%20Reference))
  (Rendering|Material|SetMaterial (Variables|Default|GetStaticMesh) 0 "/Game/Materials/Gray_2.Gray_2")
  (Rendering|Material|SetMaterial (Variables|Default|GetStaticMesh1) 0 "/Game/Materials/Gray_2.Gray_2")
  (Rendering|Material|SetMaterial (Variables|Default|GetStaticMesh2) 0 "/Game/Materials/Gray_2.Gray_2")
  (Rendering|Material|SetMaterial (Variables|Default|GetStaticMesh3) 0 "/Game/Materials/Gray_2.Gray_2"))

(event OnClicked(StaticMesh2)
  (params (TouchedComponent :type Primitive%20Component%20Object%20Reference) (ButtonPressed :type Key%20Structure))
  (Game|OpenLevel(byName) "MainMenu"))

(event OnClicked(StaticMesh3)
  (params (TouchedComponent :type Primitive%20Component%20Object%20Reference) (ButtonPressed :type Key%20Structure))
  (Game|OpenLevel(byName) "MainMenu"))

(event OnBeginCursorOver(StaticMesh2)
  (params (TouchedComponent :type Primitive%20Component%20Object%20Reference))
  (Rendering|Material|SetMaterial (Variables|Default|GetStaticMesh) 0 "/Game/Materials/Brown_10.Brown_10")
  (Rendering|Material|SetMaterial (Variables|Default|GetStaticMesh1) 0 "/Game/Materials/Brown_10.Brown_10")
  (Rendering|Material|SetMaterial (Variables|Default|GetStaticMesh2) 0 "/Game/Materials/Brown_10.Brown_10")
  (Rendering|Material|SetMaterial (Variables|Default|GetStaticMesh3) 0 "/Game/Materials/Brown_10.Brown_10"))

(event OnBeginCursorOver(StaticMesh3)
  (params (TouchedComponent :type Primitive%20Component%20Object%20Reference))
  (Rendering|Material|SetMaterial (Variables|Default|GetStaticMesh) 0 "/Game/Materials/Brown_10.Brown_10")
  (Rendering|Material|SetMaterial (Variables|Default|GetStaticMesh1) 0 "/Game/Materials/Brown_10.Brown_10")
  (Rendering|Material|SetMaterial (Variables|Default|GetStaticMesh2) 0 "/Game/Materials/Brown_10.Brown_10")
  (Rendering|Material|SetMaterial (Variables|Default|GetStaticMesh3) 0 "/Game/Materials/Brown_10.Brown_10"))

(fn ConstructionScript
  (|CallParentFunction))