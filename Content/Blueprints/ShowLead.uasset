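; ShowLead fills an in-world leaderboard with player names and scores when play begins.
; It takes the current score and name from the Global game instance, passes them to SetLeaderboard and SortLead, then reads entries back through ReadScore.
; Paired TextRender actors display each entry or hide when the name is empty, though the loop covers ten indices against five pairs.
; The button click is empty, and menu-return and resume logic is unconnected.
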(event OnClicked(Button_94))

(event EventBeginPlay
  (bind _asglobal (Utilities|Casting|CastToGlobal (Game|GetGameInstance)))
  (Utilities|Casting|CastToFirstPersonCharacterRayCast_ProhressBar (Game|GetPlayerCharacter 0))
  (Class|LeaderBoard|SetLeaderboard 0 (Variables|/Game/Blueprints/Global.Global_C|GetScore _asglobal) (Variables|/Game/Blueprints/Global.Global_C|GetPlayerName _asglobal))
  (Class|LeaderBoard|SortLead (Variables|/Game/Blueprints/Global.Global_C|GetScore _asglobal) (Variables|/Game/Blueprints/Global.Global_C|GetPlayerName _asglobal))
  (for _index (range 0 9)
    (bind (_num _name _score) (Class|LeaderBoard|ReadScore _index (Variables|/Game/Blueprints/Global.Global_C|GetPlayerName _asglobal)))
    (if (Utilities|Text|TextIsEmpty (Utilities|Text|ToText(String) _name))
      (Rendering|SetVisibility (Variables|/Script/Engine.TextRenderActor|GetTextRender (Utilities|Array|Get(acopy) (Utilities|Array|MakeArray (Variables|Default|GetText) (Variables|Default|GetText_0) (Variables|Default|GetText_1) (Variables|Default|GetText_2) (Variables|Default|GetText_3)) _index)) false false)
      (Rendering|SetVisibility (Variables|/Script/Engine.Actor|GetRootComponent (Utilities|Array|Get(acopy) (Utilities|Array|MakeArray (Variables|Default|GetText_4) (Variables|Default|GetText_5) (Variables|Default|GetText_6) (Variables|Default|GetText_7) (Variables|Default|GetText_8)) _index)) false false)
      (else
        (Rendering|Components|TextRender|SetText (Variables|/Script/Engine.TextRenderActor|GetTextRender (Utilities|Array|Get(acopy) (Utilities|Array|MakeArray (Variables|Default|GetText) (Variables|Default|GetText_0) (Variables|Default|GetText_1) (Variables|Default|GetText_2) (Variables|Default|GetText_3)) _index)) (Utilities|Text|ToText(String) _name))
        (Rendering|Components|TextRender|SetText (Variables|/Script/Engine.TextRenderActor|GetTextRender (Utilities|Array|Get(acopy) (Utilities|Array|MakeArray (Variables|Default|GetText_4) (Variables|Default|GetText_5) (Variables|Default|GetText_6) (Variables|Default|GetText_7) (Variables|Default|GetText_8)) _index)) (Utilities|Text|ToText(Integer) _score))))))

(fn ConstructionScript)